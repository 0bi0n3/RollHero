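; LaunchButton is an actor with a button that moves vertically when a BallPawn overlaps it.
; Beginning an overlap plays a kick-drum thump at the actor's location and plays a timeline, while ending the overlap reverses it.
; The timeline's ButtonLaunch value offsets the Button component's world Z from InitialButtonLocation on each update, without sweeping.
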(event `self.ReceiveBeginPlay`
  (`parent.ReceiveBeginPlay`))

(event `self.ReceiveActorBeginOverlap`
  (params (OtherActor :type "Actor Object Reference"))
  (cast `/Game/Blueprints/BallPawn` OtherActor)
  (`GameplayStatics.PlaySoundAtLocation` "/Game/Audio/WAVs/Musical__Sample__808_Kick__Boom__Sub__Thump__Short__Processed_04_SND36003.Musical__Sample__808_Kick__Boom__Sub__Thump__Short__Processed_04_SND36003" (`self.K2_GetActorLocation`) (struct) 1.0 1.0 0.0 null null null null)
  (bind (_direction _buttonlaunch) (`Timeline|ButtonLaunchTimeline` :!label _label)
    (:`Update`
      ;[0.7391 0.4582 1] Set button location.
      (`SceneComponent.K2_SetWorldLocation` (`self.Button`) (`KismetMathLibrary.MakeVector` (.x (`self.InitialButtonLocation`)) (.y (`self.InitialButtonLocation`)) (+ (.z (`self.InitialButtonLocation`)) _buttonlaunch)) false false))))

(event `self.ReceiveActorEndOverlap`
  (params (OtherActor :type "Actor Object Reference"))
  (cast `/Game/Blueprints/BallPawn` OtherActor)
  (goto _label :!via `Reverse`))

(fn `UserConstructionScript`
  (`parent.UserConstructionScript`))