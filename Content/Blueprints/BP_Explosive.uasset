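; An explosive pickup that launches the player's ball when collected and has zero base points.
; BeginPlay sets the parent pickup's explosion sound and particles, disables the number widget and starts a spark sound at its location.
; On pickup by a BallPawn, it applies a constant-falloff radial velocity impulse to the ball mesh from slightly below itself.
; It then stops the sparks and calls the parent pickup logic.
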(event `self.ReceiveBeginPlay`
  (set `self.UseNumberWidget` false)
  (set `self.BasePoints` 0)
  (set `self.OnPickupSound` "/Game/StarterContent/Audio/Explosion01.Explosion01")
  (set `self.OnPickupParticles` "/Game/InfinityBladeEffects/Effects/FX_Monsters/FX_Monster_Gruntling/Bomber/P_FireBombExplosion.P_FireBombExplosion")
  (bind _returnvalue (`GameplayStatics.SpawnSoundAtLocation` "/Game/StarterContent/Audio/Fire_Sparks01_Cue.Fire_Sparks01_Cue" (`self.K2_GetActorLocation`) (struct) 1.0 1.0 0.0 null null))
  (set `self.Spark Sound` _returnvalue)
  (`parent.ReceiveBeginPlay`))

(event `self.OnPickup`
  (params (`Other Actor` :type "Object Object Reference"))
  (bind _asball_pawn (cast `/Game/Blueprints/BallPawn` `Other Actor`))
  (`PrimitiveComponent.AddRadialImpulse` (`/Game/Blueprints/BallPawn.BallMesh` _asball_pawn) (`KismetMathLibrary.MakeVector` (.x (`self.K2_GetActorLocation`)) (.y (`self.K2_GetActorLocation`)) (+ (.z (`self.K2_GetActorLocation`)) -50.0)) 500.0 3000.0 "RIF_Constant" true)
  (`AudioComponent.Stop` (`self.Spark Sound`))
  (`parent.OnPickup` `Other Actor`))

(fn `UserConstructionScript`
  (`parent.UserConstructionScript`))